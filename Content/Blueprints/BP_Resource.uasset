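; BP_Resource is a harvestable resource actor that players wear down to gain resources.
; Harvest creates a progress widget on the player's HUD on first hit, then CheckProgress subtracts the harvest amount from its current life and updates the bar.
; At zero life it removes the widget, adds a random amount within MaterialDropChance to the player's Resources and destroys itself.
; Stopping harvesting removes the widget but keeps the remaining life.
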(event `/Game/Blueprints/BPI_Resource_Interactions.Harvest`
  (params (harvestAmount :type "Float (single-precision)") (PlayerRef :type "/Game/ThirdPersonCPP/Blueprints/ThirdPersonCharacter Object Reference"))
  (set `self.playerRef` PlayerRef)
  (if (`KismetSystemLibrary.IsValid` (`self.harvestUIRef`))
    (`self.CheckProgress` harvestAmount)
    (else
      (bind _returnvalue (`|CreateWidget` "/Game/Blueprints/Harvest_UI.Harvest_UI_C"))
      (bind _output_get (set `self.harvestUIRef` _returnvalue))
      (bind _returnvalue_2 (`PanelWidget.AddChild` (`/Game/Blueprints/HUD_UI.MainPanel` (`/Game/ThirdPersonCPP/Blueprints/ThirdPersonCharacter.hudRef` (`self.playerRef`))) _output_get))
      (bind _ascanvas_panel_slot (cast `CanvasPanelSlot` _returnvalue_2))
      (`CanvasPanelSlot.SetAnchors` _ascanvas_panel_slot (make `Anchors` (0.4 0.8) (0.6 0.87)))
      (`CanvasPanelSlot.SetPosition` _ascanvas_panel_slot (0.0 0.0))
      (`CanvasPanelSlot.SetSize` _ascanvas_panel_slot (0.0 0.0))
      (`self.CheckProgress` harvestAmount))))

(event `/Game/Blueprints/BPI_Resource_Interactions.UserStoppedHarvesting`
  (`Widget.RemoveFromParent` (`self.harvestUIRef`))
  (set `self.harvestUIRef` null))

(fn `CheckProgress`
  (params (harvestAmount :type "Float (double-precision)"))
  (bind _output_get (set `self.harvestCurrentLife` (- (`self.harvestCurrentLife`) harvestAmount)))
  (if (<= _output_get 0.0)
    (`self.ResourceDepleted`)
    (else
      (`/Game/Blueprints/Harvest_UI.UpdateProgress` (`self.harvestUIRef`) (`self.harvestCurrentLife`) (`self.harvestMaxLife`)))))

(fn `ResourceDepleted`
  (bind _playerref (`self.playerRef`))
  (bind _materialdropchance (`self.materialDropChance`))
  (`Widget.RemoveFromParent` (`self.harvestUIRef`))
  (set `/Game/ThirdPersonCPP/Blueprints/ThirdPersonCharacter.resources` (+ (`/Game/ThirdPersonCPP/Blueprints/ThirdPersonCharacter.resources` _playerref) (`KismetMathLibrary.RandomIntegerInRange` (`|GetArrayItem` _materialdropchance) (`|GetArrayItem` _materialdropchance 1))) _playerref)
  (`self.K2_DestroyActor`))

(fn `UserConstructionScript`)